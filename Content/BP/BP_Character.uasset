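; BP_Character is a character Blueprint that provides basic player movement and look control through Enhanced Input.
; On BeginPlay it adds the IMC_BaseCharacter mapping context to the local player subsystem of player controller 0.
; Locomotion and strafe actions add movement input along the actor's forward and right vectors, while separate vertical and horizontal look actions drive controller pitch and yaw.
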(event `self.ReceiveBeginPlay`
  ;[1 1 1] Establish IMC Mapping
  (`EnhancedInputSubsystemInterface.AddMappingContext` (pcsubsystem `EnhancedInputLocalPlayerSubsystem` (`GameplayStatics.GetPlayerController` 0)) "/Game/BP/UI/IO/IMC_BaseCharacter.IMC_BaseCharacter" 0 (struct)))

(event `EnhancedInput|/Game/BP/UI/IO/IA_Locomotion`
  (params (ActionValue :type "Float (double-precision)") (ElapsedSeconds :type "Float (double-precision)") (TriggeredSeconds :type "Float (double-precision)") (InputAction :type "InputAction Object Reference" :default "/Game/BP/UI/IO/IA_Locomotion.IA_Locomotion"))
  ;[1 1 1] Basic Input
  (:`Triggered`
    (`self.AddMovementInput` (`self.GetActorForwardVector`) ActionValue)))

(event `EnhancedInput|/Game/BP/UI/IO/IA_Strafe`
  (params (ActionValue :type "Float (double-precision)") (ElapsedSeconds :type "Float (double-precision)") (TriggeredSeconds :type "Float (double-precision)") (InputAction :type "InputAction Object Reference" :default "/Game/BP/UI/IO/IA_Strafe.IA_Strafe"))
  ;[1 1 1] Basic Input
  (:`Triggered`
    (`self.AddMovementInput` (`self.GetActorRightVector`) ActionValue)))

(event `EnhancedInput|/Game/BP/UI/IO/IA_LookV`
  (params (ActionValue :type "Float (double-precision)") (ElapsedSeconds :type "Float (double-precision)") (TriggeredSeconds :type "Float (double-precision)") (InputAction :type "InputAction Object Reference" :default "/Game/BP/UI/IO/IA_LookV.IA_LookV"))
  ;[1 1 1] Basic Input
  (:`Triggered`
    (`self.AddControllerPitchInput` ActionValue)))

(event `EnhancedInput|/Game/BP/UI/IO/IA_LookH`
  (params (ActionValue :type "Float (double-precision)") (ElapsedSeconds :type "Float (double-precision)") (TriggeredSeconds :type "Float (double-precision)") (InputAction :type "InputAction Object Reference" :default "/Game/BP/UI/IO/IA_LookH.IA_LookH"))
  ;[1 1 1] Basic Input
  (:`Triggered`
    (`self.AddControllerYawInput` ActionValue)))

(fn `UserConstructionScript`)